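; BP_Camera is a standalone camera actor that follows the player's BP_FighterMan pawn.
; On BeginPlay it caches that pawn, enables following and makes itself the player controller's view target.
; While following, each Tick lerps its location toward the player's using delta seconds times Speed, giving a smoothed chase without sweep collision.
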(event EventBeginPlay
  (bind _asbp_fighter_man (Utilities|Casting|CastToBP_FighterMan (Game|Player|GetPlayerPawn 0)))
  (Variables|Default|SetPlayer _asbp_fighter_man)
  (Variables|Default|SetFollow true)
  (Game|Player|SetViewTargetwithBlend (Game|GetPlayerController 0) self 0.0 "VTBlend_Linear" 0.0 false))

(event Collision|EventActorBeginOverlap
  (params (OtherActor :type Actor%20Object%20Reference)))

(event EventTick
  (params (DeltaSeconds :type Float%20%28single-precision%29))
  (if (Variables|Default|GetFollow)
    (CallFunction|MovCamera)))

(fn ConstructionScript)

(fn MovCamera
  (bind _returnvalue (Transformation|GetActorLocation))
  (bind _player (Variables|Default|GetPlayer))
  (bind _returnvalue_2 (Transformation|GetActorLocation _player))
  (Transformation|SetActorLocation (Math|Vector|Lerp(Vector) (Math|Vector|MakeVector (.x _returnvalue) (.y _returnvalue) (.z _returnvalue)) (Math|Vector|MakeVector (.x _returnvalue_2) (.y _returnvalue_2) (.z _returnvalue_2)) (* (Utilities|Time|GetWorldDeltaSeconds) (Variables|Default|GetSpeed))) false false))